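; Spawner actor that fills the aquarium with creatures and swaps the population when the geological period changes.
; On BeginPlay it picks a preferred region, taken from the AR pawn's attachment if one exists, then spawns CreatureList.
; PeriodUpdated rebuilds that list from CreatureTable, filtering by period rarity and randomizing group sizes.
; Each spawn pass destroys every BP_Creature, then places new ones randomly in a box above the spawner.
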(event Custom|Spawn%20Configured%20Creatures
  (bind _outactors (Actor|GetAllActorsOfClass "/Game/Creatures/BP_Creature.BP_Creature_C"))
  (for _array_element _outactors
    (Actor|DestroyActor _array_element))
  (for _array_element_2 (Variables|Default|GetCreatureList)
    (bind _returnvalue (Utilities|GetDataTableRow (.DataTable (Utilities|Struct|BreakDataTableRowHandle (.Creature (Utilities|Struct|BreakStruct_CreatureSpawnParams _array_element_2)))) (.RowName (Utilities|Struct|BreakDataTableRowHandle (.Creature (Utilities|Struct|BreakStruct_CreatureSpawnParams _array_element_2)))))
      (:then
        (for _index (range 0 (.Quantity (Utilities|Struct|BreakStruct_CreatureSpawnParams _array_element_2)))
          (Game|SpawnActorfromClass :Class (.Class (Utilities|Struct|BreakCreatureStructure _returnvalue)) :SpawnTransform (Math|Transform|MakeTransform (+ (Math|Random|RandomPointinBoundingBox "0, 0,1000.000000" "1000.000000,1000.000000,500.000000") (Transformation|GetWorldLocation (Variables|Default|GetDefaultSceneRoot)))) :CollisionHandlingOverride "Undefined" :TargetObject 0 :PreferredRegion (.PreferredRegion (Utilities|Struct|BreakStruct_CreatureSpawnParams _array_element_2)) :Instigator 0))))))

(event Custom|Period%20Updated
  (params (NewPeriod :type Enum_Periods%20Enum :default "NewEnumerator0"))
  (bind _output_get (Variables|Default|SetActivePeriod NewPeriod))
  (Variables|Default|SetCreatureList (CallFunction|CreateCreatureListBasedonSingleEra _output_get))
  (CallFunction|SpawnConfiguredCreatures))

(event EventBeginPlay
  (Utilities|FlowControl|Sequence
    (:then_0
      ;[1 1 1] If there's an AR pawn, the preferred region becomes the region all creatures target.
      (bind _returnvalue (Actor|GetActorOfClass "/Game/AR/BP_ARPawn.BP_ARPawn_C"))
      (Utilities|IsValid _returnvalue
        (:Is%20Valid
          (bind _asbp_aquarium_regions (Utilities|Casting|CastToBP_AquariumRegions (Utilities|Array|Get(acopy) (Actor|GetAttachedActors _returnvalue true))))
          (bind _output_get (Variables|Default|SetPreferredRegionTEMP _asbp_aquarium_regions))
          (for _array_element (Variables|Default|GetCreatureList)
            (Utilities|Struct|SetmembersinStruct_CreatureSpawnParams _array_element _output_get)))
        (:Is%20Not%20Valid
          (Variables|Default|SetPreferredRegionTEMP (.PreferredRegion (Utilities|Struct|BreakStruct_CreatureSpawnParams (Utilities|Array|Get(acopy) (Variables|Default|GetCreatureList))))))))
    (:then_1
      (CallFunction|SpawnConfiguredCreatures))))

(fn ConstructionScript
  (Variables|Default|SetAllSpawnableAnimals (CallFunction|CreateCreatureListBasedonEntireTable)))

(fn CreateCreatureListBasedonEntireTable
  (bind _outrownames (DataTable|GetDataTableRowNames "/Game/Creatures/CreatureTable.CreatureTable"))
  (for _array_element _outrownames
    (bind _returnvalue (Utilities|GetDataTableRow "/Game/Creatures/CreatureTable.CreatureTable" _array_element)
      (:then
        (if (and (> (.X (Math|Vector2D|BreakVector2D (.GroupValues (Utilities|Struct|BreakCreatureStructure _returnvalue)))) 0.0) (Utilities|IsValidClass (.Class (Utilities|Struct|BreakCreatureStructure _returnvalue))))
          (Utilities|Array|Add (LocalVariables|GetList) (Utilities|Struct|MakeStruct_CreatureSpawnParams (Utilities|Struct|MakeDataTableRowHandle "/Game/Creatures/CreatureTable.CreatureTable" _array_element) (Math|Random|RandomIntegerinRange (- (Math|Float|Truncate (.X (Math|Vector2D|BreakVector2D (.GroupValues (Utilities|Struct|BreakCreatureStructure _returnvalue))))) (Math|Float|Truncate (.Y (Math|Vector2D|BreakVector2D (.GroupValues (Utilities|Struct|BreakCreatureStructure _returnvalue)))))) (+ (Math|Float|Truncate (.X (Math|Vector2D|BreakVector2D (.GroupValues (Utilities|Struct|BreakCreatureStructure _returnvalue))))) (Math|Float|Truncate (.Y (Math|Vector2D|BreakVector2D (.GroupValues (Utilities|Struct|BreakCreatureStructure _returnvalue))))))) (Variables|Default|GetPreferredRegionTEMP)))))))
  (return (LocalVariables|GetList)))

(fn CreateCreatureListBasedonSingleEra
  (params (Period :type Enum_Periods%20Enum :default "NewEnumerator0"))
  (if (Utilities|Enum|NotEqual(Enum) Period "NewEnumerator0")
    (bind _outrownames (DataTable|GetDataTableRowNames "/Game/Creatures/CreatureTable.CreatureTable"))
    (for _array_element _outrownames
      (bind _returnvalue (Utilities|GetDataTableRow "/Game/Creatures/CreatureTable.CreatureTable" _array_element)
        (:then
          (if (Math|Boolean|ANDBoolean (> (.X (Math|Vector2D|BreakVector2D (.GroupValues (Utilities|Struct|BreakCreatureStructure _returnvalue)))) 0.0) (Utilities|IsValidClass (.Class (Utilities|Struct|BreakCreatureStructure _returnvalue))) (> (Utilities|Array|Get(acopy) (.Rarity (Utilities|Struct|BreakCreatureStructure _returnvalue)) (Utilities|Select :Index Period :NewEnumerator0 0 :NewEnumerator1 0 :NewEnumerator2 1 :NewEnumerator3 2 :NewEnumerator4 3 :NewEnumerator5 4 :NewEnumerator6 5 :NewEnumerator7 6 :NewEnumerator8 7)) 0))
            (Utilities|Array|Add (LocalVariables|GetList) (Utilities|Struct|MakeStruct_CreatureSpawnParams (Utilities|Struct|MakeDataTableRowHandle "/Game/Creatures/CreatureTable.CreatureTable" _array_element) (Math|Random|RandomIntegerinRange (- (Math|Float|Truncate (.X (Math|Vector2D|BreakVector2D (.GroupValues (Utilities|Struct|BreakCreatureStructure _returnvalue))))) (Math|Float|Truncate (.Y (Math|Vector2D|BreakVector2D (.GroupValues (Utilities|Struct|BreakCreatureStructure _returnvalue)))))) (+ (Math|Float|Truncate (.X (Math|Vector2D|BreakVector2D (.GroupValues (Utilities|Struct|BreakCreatureStructure _returnvalue))))) (Math|Float|Truncate (.Y (Math|Vector2D|BreakVector2D (.GroupValues (Utilities|Struct|BreakCreatureStructure _returnvalue))))))) (Variables|Default|GetPreferredRegionTEMP)))))))
    (return (LocalVariables|GetList))
    (else
      (return (CallFunction|CreateCreatureListBasedonEntireTable)))))