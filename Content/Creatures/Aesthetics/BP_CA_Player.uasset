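; Player creature aesthetics Blueprint that animates a squid body and shell from its parent's movement.
; Each tick, while the parent is valid, it pitches the Shell further as movement speed rises.
; It also grows PercentMaxSpeed cumulatively from the length of movement velocity plus actor velocity.
; The same combined velocity drives the squid skeleton's SiphonClosed morph target, opening the siphon as speed increases.
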(event EventTick
  (params (DeltaSeconds :type Float%20%28single-precision%29))
  (bind _parent (Variables|Default|GetParent))
  (bind _returnvalue (Transformation|GetVelocity _parent))
  (bind _movementcomponent (Variables|/Game/Creatures/BP_Creature.BP_Creature_C|GetMovementComponent _parent))
  (bind _velocity (Variables|/Script/Engine.MovementComponent|GetVelocity _movementcomponent))
  (bind _returnvalue_2 (+ _velocity _returnvalue))
  (bind _returnvalue_3 (Math|Vector|VectorLength _returnvalue_2))
  (|CallParentFunction DeltaSeconds)
  (Utilities|IsValid (Variables|Default|GetParent)
    (:Is%20Valid
      (Utilities|FlowControl|Sequence
        (:then_0
          (Transformation|SetRelativeRotation (Variables|Default|GetShell) (Math|Rotator|MakeRotator -9e+01 (Math|Float|MapRangeClamped (Math|Vector|VectorLength _velocity) 0.0 3e+02 -6e+01 -85.0) 1.8e+02) false false)
          (Variables|Default|SetPercentMaxSpeed (+ (Variables|Default|GetPercentMaxSpeed) (* _returnvalue_3 0.001))))
        (:then_1
          (Components|SkeletalMesh|SetMorphTarget (Variables|Default|GetSquidSkeleton) "SiphonClosed" (Math|Float|MapRangeClamped _returnvalue_3 0.0 5e+02 1.0 0.0) true))))))

(fn ConstructionScript
  (|CallParentFunction))