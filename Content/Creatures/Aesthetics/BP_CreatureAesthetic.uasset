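; BP_CreatureAesthetic is the aesthetic actor for a BP_Creature, with a text label and measured motion values.
; On Tick it retries until an Instigator exists, then caches it once as Parent if it is a creature.
; It turns the label toward the player camera and allows its text to be set.
; From Parent it derives speed fraction, vertical velocity and per-frame yaw change, not scaled by delta time.
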(event Custom|Set%20Label%20Text
  (params (New%20Text :type String))
  (Rendering|Components|TextRender|SetText (Variables|Default|GetLabel) (Utilities|Text|ToText(String) New%20Text)))

(event EventBeginPlay)

(event EventTick
  (params (DeltaSeconds :type Float%20%28single-precision%29))
  (bind _returnvalue (Game|GetInstigator))
  (bind _label (Variables|Default|GetLabel))
  (Utilities|FlowControl|Sequence
    (:then_0
      ;[1 1 1] Parent Setup
      (Utilities|FlowControl|DoOnce false :!label _label
        (:Completed
          (Utilities|IsValid _returnvalue
            (:Is%20Valid
              (bind _asbp_creature (Utilities|Casting|CastToBP_Creature _returnvalue)) ; If cast failed, we got a parent but it wasn't a Creature.
              (Variables|Default|SetParent _asbp_creature))
            (:Is%20Not%20Valid
              (goto _label Reset))))))
    (:then_1
      ;[1 1 1] Make Label Follow Camera
      (Transformation|SetWorldRotation _label (Math|Rotator|FindLookatRotation (Transformation|GetWorldLocation _label) (Camera|GetCameraLocation (Game|GetPlayerCameraManager 0))) false false))
    (:then_2
      ;[1 1 1] Measure Speeds
      (Utilities|IsValid (Variables|Default|GetParent)
        (:Is%20Valid
          (Variables|Default|SetPercentMaxSpeed (/ (Math|Vector|VectorLength (Variables|/Script/Engine.MovementComponent|GetVelocity (Pawn|GetMovementComponent (Variables|Default|GetParent)))) (Class|MovementComponent|GetMaxSpeed (Pawn|GetMovementComponent (Variables|Default|GetParent)))))
          (Variables|Default|SetVelocityVertical (.Z (Math|Vector|BreakVector (Variables|/Script/Engine.MovementComponent|GetVelocity (Pawn|GetMovementComponent (Variables|Default|GetParent))))))
          (Variables|Default|SetVelocityYaw (- (.Yaw (Default|GetEulerAngles (Variables|Default|GetParent) (Transformation|GetWorldRotation (Variables|/Game/Creatures/BP_Creature.BP_Creature_C|GetCollision (Variables|Default|GetParent))))) (Variables|Default|GetYawLastFrame)))
          (Variables|Default|SetYawLastFrame (.Yaw (Default|GetEulerAngles (Variables|Default|GetParent) (Transformation|GetWorldRotation (Variables|/Game/Creatures/BP_Creature.BP_Creature_C|GetCollision (Variables|Default|GetParent)))))))))))

(fn ConstructionScript)