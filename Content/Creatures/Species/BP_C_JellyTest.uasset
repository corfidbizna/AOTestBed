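; BP_C_JellyTest is a test Blueprint for a jelly creature that configures the material on its Jelly component.
; The construction script creates a dynamic material instance from slot 0 and sets its start and end distance parameters.
; Setters for displacement, retraction, phase frequency and ripple offset are disconnected, and the event graph holds only disabled default events.
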(event EventBeginPlay
  (|CallParentFunction) ; This node is disabled and will not be called.\nDrag off pins to build functionality.
)

(event Collision|EventActorBeginOverlap
  (params (OtherActor :type Actor%20Object%20Reference)))

(event EventTick
  (params (DeltaSeconds :type Float%20%28single-precision%29))
  (|CallParentFunction DeltaSeconds) ; This node is disabled and will not be called.\nDrag off pins to build functionality.
)

(fn ConstructionScript
  (bind _jelly (Variables|Default|GetJelly))
  (|CallParentFunction)
  (bind _returnvalue (Rendering|Material|CreateDynamicMaterialInstance _jelly 0 (Rendering|Material|GetMaterial _jelly 0) "None" :!class /Script/Engine.PrimitiveComponent))
  (Rendering|Material|SetScalarParameterValue _returnvalue "Start Distance" 0.0 :!class /Script/Engine.MaterialInstanceDynamic)
  (Rendering|Material|SetScalarParameterValue _returnvalue "End Distance" 6e+01 :!class /Script/Engine.MaterialInstanceDynamic) ; 50
)