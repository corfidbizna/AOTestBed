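; Physics-driven creature that moves through 3D space with buoyancy-like vertical input, configured from a creature data table that supplies stats and an optional attached visual actor.
; It follows a target object or periodically repaths to random, region or requested points.
; Tick steers with mass-scaled PID torques on yaw, pitch and roll, then propels it by steady input or timed impulses when facing the target.
; It also handles distance-threshold events, creature bumps, damage and a camera-facing label.
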(event Custom|Repath%20new%20point
  (bind _preferredregion (Variables|Default|GetPreferredRegion))
  ;[1 1 1 1 15] This is so that if no one is listening to "Request New Point" it still will have somewhere new to go.
  (CallFunction|MoveTowardsPoint (Math|Random|RandomPointinBoundingBox "0, 0,100.000000" "400.000000,400.000000,200.000000"))
  (Utilities|IsValid _preferredregion
    (:Is%20Valid
      (bind _point (Default|GetPointInsideCoordinateBounds _preferredregion))
      (CallFunction|MoveTowardsPoint _point))
    (:Is%20Not%20Valid
      (Default|CallRequestNewPoint self (Variables|Default|GetTargetPoint))))
  (Utilities|FlowControl|Delay (Math|Random|RandomFloatinRange 5.0 1e+01))
  (CallFunction|RepathNewPoint))

(event EventBeginPlay
  (bind _self self)
  (bind _creaturetableentry (Variables|Static|GetCreatureTableEntry))
  (bind (_datatable _rowname) (Utilities|Struct|BreakDataTableRowHandle _creaturetableentry))
  (if (Variables|Default|GetUseAesthetic)
    (bind _returnvalue (Utilities|GetDataTableRow _datatable _rowname)
      (:then
        (bind _returnvalue_2 (Game|SpawnActorfromClass (.Mesh (Utilities|Struct|BreakCreatureStructure _returnvalue)) (Math|Transform|MakeTransform "0, 0, 0") "Undefined" _self _self))
        (bind _output_get (Variables|Default|SetCreatureAesthetic _returnvalue_2))
        (Collision|IgnoreActorwhenMoving (Variables|Default|GetCollision) _output_get true)
        (Transformation|AttachActorToActor _output_get self "None" "KeepRelative" "KeepRelative" "KeepRelative" false)
        (Default|SetLabelText _output_get (Utilities|String|ToString(Name) (Variables|Static|GetCreatureName)))))))

(event EventTick
  (params (DeltaSeconds :type Float%20%28single-precision%29))
  (bind _returnvalue (Utilities|Time|GetWorldDeltaSeconds))
  (bind _returnvalue_2 (Utilities|Time|GetWorldDeltaSeconds))
  (bind _returnvalue_3 (Utilities|Time|GetWorldDeltaSeconds))
  (bind _returnvalue_4 (Math|Float|MakeLiteralFloat 4e+01))
  (bind _returnvalue_5 (Utilities|TargetPointRelative))
  (bind _returnvalue_6 (Utilities|TargetPointRelative))
  (bind _returnvalue_7 (Utilities|TargetPointRelative))
  (bind _self self)
  (bind _collision (Variables|Default|GetCollision))
  (bind _collision_2 (Variables|Default|GetCollision))
  (bind _collision_3 (Variables|Default|GetCollision))
  (bind _targetobject (Variables|Default|GetTargetObject))
  (bind _collision_4 (Variables|Default|GetCollision))
  (bind _movementinputfrequency (Variables|Static|GetMovementInputFrequency))
  (bind _distancetotargetmargins (Variables|Constant|GetDistanceToTargetMargins))
  (bind _pitchcap (Variables|Default|GetPitchCap))
  (bind _movementcomponent (Variables|Default|GetMovementComponent))
  (bind _movementcomponent_2 (Variables|Default|GetMovementComponent))
  (bind _label (Variables|Default|GetLabel))
  (bind _collision_5 (Variables|Default|GetCollision))
  (bind _returnvalue_8 (Transformation|GetWorldRotation _collision_4))
  (bind _returnvalue_9 (Math|Conversions|ToVector2D(Vector) _returnvalue_6))
  (bind _returnvalue_10 (Transformation|GetWorldRotation _collision_2))
  (bind _returnvalue_11 (Transformation|GetWorldRotation _collision_3))
  (bind _returnvalue_12 (Math|Float|Power 0.2 _returnvalue_3))
  (bind _returnvalue_13 (Math|Conversions|ToVector2D(Vector) _returnvalue_5))
  (bind (_x _y _z) (Math|Vector|BreakVector _returnvalue_7))
  (bind _returnvalue_14 (Transformation|GetWorldRotation _collision))
  (bind _returnvalue_15 (Transformation|GetActorForwardVector _self))
  (bind _returnvalue_16 (* _movementinputfrequency 0.25))
  (bind _out (Utilities|*-1 _returnvalue_4))
  (bind _velocity (Variables|/Script/Engine.MovementComponent|GetVelocity _movementcomponent))
  (bind _velocity_2 (Variables|/Script/Engine.MovementComponent|GetVelocity _movementcomponent_2))
  (bind _sphereradius (Variables|/Script/Engine.SphereComponent|GetSphereRadius _collision_5))
  (bind _yaw (CallFunction|GetEulerAngles _returnvalue_14))
  (bind (_roll _pitch _yaw_2 _pitch_torque_axis _roll_torque_axis) (CallFunction|GetEulerAngles _returnvalue_11))
  (bind _yaw_3 (CallFunction|GetEulerAngles _returnvalue_8))
  (bind _returnvalue_17 (Math|Vector2D|Normalize2D _returnvalue_9))
  (bind (_roll_2 _pitch_2 _yaw_4) (Math|Rotator|BreakRotator _returnvalue_10))
  (bind _returnvalue_18 (* _returnvalue_15 _returnvalue))
  (bind _returnvalue_19 (- 1.0 _returnvalue_12))
  (bind _returnvalue_20 (Math|Vector2D|Vector2DLength _returnvalue_13))
  (bind _returnvalue_21 (Math|Conversions|ToVector2D(Vector) _returnvalue_15))
  (bind _returnvalue_22 (* _distancetotargetmargins _sphereradius))
  (bind _returnvalue_23 (Math|Vector|Normalize _returnvalue_18))
  (bind _returnvalue_24 (Math|Vector2D|DotProduct(2D) _returnvalue_17 _returnvalue_21))
  (bind _returnvalue_25 (* _returnvalue_22 2.0))
  (bind (_x_2 _y_2) (Math|Vector2D|BreakVector2D _returnvalue_25))
  (bind _returnvalue_26 (> _returnvalue_24 0.8))
  (Utilities|FlowControl|Sequence
    (:then_0
      ;[1 1 1] Make Label Face Camera
      (Transformation|SetWorldRotation _label (Math|Rotator|FindLookatRotation (Transformation|GetWorldLocation _label) (Camera|GetCameraLocation (Game|GetPlayerCameraManager 0))) false false))
    (:then_1
      ;[1 1 1] Follow Target if Present
      (Utilities|IsValid _targetobject
        (:Is%20Valid
          (CallFunction|MoveTowardsPoint (Transformation|GetWorldLocation (Variables|/Script/Engine.Actor|GetRootComponent _targetobject)))
          (Variables|Movement|SetPercentMaxSpeed (/ (Math|Vector|VectorLength _velocity_2) (Class|MovementComponent|GetMaxSpeed _movementcomponent_2)))
          (Variables|Movement|SetVelocityVertical (.Z (Math|Vector|BreakVector _velocity_2)))
          (Variables|Movement|SetVelocityYaw (- _yaw (Variables|Movement|GetYawLastFrame)))
          (Variables|Movement|SetYawLastFrame _yaw))))
    (:then_2
      ;[1 1 1] Translation
      (Utilities|FlowControl|Sequence
        (:then_0
          ;;[1 1 1] Baseline Vertical (Buoyancy)
          (Class|PawnMovementComponent|AddInputVector (Variables|Default|GetMovementComponent) (Math|Vector|MakeVector 0.0 0.0 (* (Math|Float|MapRangeClamped (.Z (Math|Vector|BreakVector (Utilities|TargetPointRelative))) -1e+02 1e+02 -1.0 1.0) (Math|Float|MakeLiteralFloat 0.65))) false))
        (:then_1
          (if (Variables|Default|GetIs%20Translating)
            ;;[1 1 1] Towards While Facing
            (if (<= (Variables|Static|GetMovementInputFrequency) 0.0)
              (if _returnvalue_26
                (Class|PawnMovementComponent|AddInputVector (Variables|Default|GetMovementComponent) _returnvalue_23 false))
              (elif (< _movementinputfrequency (Variables|Default|GetMovementInputCooldown))
                (Variables|Default|SetMovementInputCooldown (Math|Random|RandomFloatinRange (* _returnvalue_16 -1.0) _returnvalue_16))
                (if _returnvalue_26
                  (Physics|AddImpulse (Variables|Default|GetCollision) (* (* _returnvalue_23 (Variables|Static|GetMovementInputFrequency)) 1e+02) "None" true))
                (else
                  (Variables|Default|SetMovementInputCooldown (+ (Variables|Default|GetMovementInputCooldown) _returnvalue)))))))))
    (:then_3
      ;[1 1 1] Steering Set-up
      (if (and (Variables|Default|GetIs%20Rotating) (> (Math|Vector|VectorLengthSquared (Utilities|TargetPointRelative)) 1e+02))
        (Utilities|FlowControl|Sequence
          (:then_0
            (Variables|Default|SetDesiredRotations (Math|Vector|MakeVector 0.0 (Math|Float|Clamp(Float) (Class|KismetMathLibrary|DegAtan2 _z (Math|Vector2D|Vector2DLength (Math|Vector2D|MakeVector2D _x _y))) (Utilities|*-1 _pitchcap) _pitchcap) (Class|KismetMathLibrary|DegAtan2 _y _x)))
            (if true :!label _label ; True evaluates to Torque-Based Steering. \nFalse evaluates to Just-Do-It Steering.
              ;[1 1 1] Torque-Based Steering
              (Utilities|FlowControl|Sequence
                (:then_0
                  (bind _oomph (Default|Tick (Variables|Default|GetPID_Yaw) (Math|Float|MapRangeClamped (CallFunction|AngleDelta (.Z (Math|Vector|BreakVector (Variables|Default|GetDesiredRotations))) _yaw_2) _out _returnvalue_4 _out _returnvalue_4) _returnvalue_2))
                  (Class|PrimitiveComponent|AddTorqueinDegrees (Variables|Default|GetCollision) (Math|Vector|MakeVector 0.0 0.0 _oomph) "None" false))
                (:then_1
                  (bind _oomph_2 (Default|Tick (Variables|Default|GetPID_Pitch) (CallFunction|AngleDelta (.Y (Math|Vector|BreakVector (Variables|Default|GetDesiredRotations))) _pitch) _returnvalue_2))
                  (Class|PrimitiveComponent|AddTorqueinDegrees (Variables|Default|GetCollision) (* _pitch_torque_axis (Utilities|*-1 _oomph_2)) "None" false))
                (:then_2
                  (bind _oomph_3 (Default|Tick (Variables|Default|GetPID_Roll) (CallFunction|AngleDelta (.X (Math|Vector|BreakVector (Variables|Default|GetDesiredRotations))) _roll) _returnvalue_2))
                  (Class|PrimitiveComponent|AddTorqueinDegrees (Variables|Default|GetCollision) (* _roll_torque_axis (Utilities|*-1 _oomph_3)) "None" false)))
              (else
                ;[1 1 1] Just-Do-It Steering
                (Transformation|SetWorldRotation (Variables|Default|GetCollision) (Math|Rotator|MakeRotator 0.0 (CallFunction|LerpAngle _pitch_2 (.Y (Math|Vector|BreakVector (Variables|Default|GetDesiredRotations))) _returnvalue_19) (CallFunction|LerpAngle _yaw_4 (.Z (Math|Vector|BreakVector (Variables|Default|GetDesiredRotations))) _returnvalue_19)) false false))))
          (:then_1
            (goto _label_2 Reset)))
        (else
          (Utilities|FlowControl|Sequence
            (:then_0
              (Utilities|FlowControl|DoOnce false :!label _label_2
                (:Completed
                  (Variables|Default|SetDesiredRotations (Math|Vector|MakeVector 0.0 0.0 (.Yaw (Math|Rotator|BreakRotator (Transformation|GetWorldRotation (Variables|Default|GetForward)))))))))
            (:then_1
              (goto _label))))))
    (:then_4
      ;[1 1 1] Nearness and Farness Check
      (if (<= _returnvalue_20 _x_2)
        (Variables|Default|SetIs%20Translating false)
        (Variables|Default|SetIs%20Rotating false)
        (Utilities|FlowControl|DoOnce false :!label _label_3
          (:Completed
            (Default|CallTargetNearThreshold)
            (goto _label_4 Reset)))
        (elif (>= _returnvalue_20 _y_2)
          (Variables|Default|SetIs%20Translating true)
          (Variables|Default|SetIs%20Rotating true)
          (Utilities|FlowControl|DoOnce false :!label _label_4
            (:Completed
              (Default|CallTargetFarThreshold)
              (goto _label_3 Reset))))))
    (:then_5
      (Variables|Movement|SetPercentMaxSpeed (/ (Math|Vector|VectorLength _velocity) (Class|MovementComponent|GetMaxSpeed _movementcomponent)))
      (Variables|Movement|SetVelocityVertical (.Z (Math|Vector|BreakVector _velocity)))
      (Variables|Movement|SetVelocityYaw (- _yaw_3 (Variables|Movement|GetYawLastFrame)))
      (Variables|Movement|SetYawLastFrame _yaw_3))
    (:then_6
      (Utilities|FlowControl|DoOnce false
        (:Completed
          (CallFunction|RepathNewPoint))))))

(event OnComponentHit(Collision)
  (params (HitComponent :type Primitive%20Component%20Object%20Reference) (OtherActor :type Actor%20Object%20Reference) (OtherComp :type Primitive%20Component%20Object%20Reference) (NormalImpulse :type Vector :default "0, 0, 0") (Hit :type Hit%20Result%20Structure%20%28by%20ref%29))
  (bind _asbp_creature (Utilities|Casting|CastToBP_Creature OtherActor))
  (Physics|AddImpulse (Variables|BP_Creature_C|GetCollision _asbp_creature) (* (.Normal (Collision|BreakHitResult Hit)) (* (Math|Float|MakeLiteralFloat -5e+01) (Math|Vector|VectorLength (Variables|/Script/Engine.MovementComponent|GetVelocity (Variables|Default|GetMovementComponent))))) "None" false))

(event Custom|Receive%20Damage
  (params (Source :type BP%20Creature%20Object%20Reference) (Amount :type Float%20%28single-precision%29))
  (bind _output_get (Variables|Default|SetHealth (- (Variables|Default|GetHealth) Amount)))
  (if (<= _output_get 0.0)
    (Default|CallOnDeath)))

(event Custom|Move%20Towards%20Point
  (params (World%20Point%20Destination :type Vector))
  (Variables|Default|SetTargetPoint World%20Point%20Destination))

(fn ConstructionScript
  (bind _returnvalue (Utilities|Name|MakeLiteralName "Behavior"))
  (bind _self self)
  (bind _returnvalue_2 (AI|GetBlackboard _self))
  (Utilities|FlowControl|Sequence
    (:then_0
      (CallFunction|CreatureStatsSetup))
    (:then_1
      (Utilities|SetUpPIDs (Variables|Default|GetPID_Roll))
      (Utilities|SetUpPIDs (Variables|Default|GetPID_Pitch))
      (Utilities|SetUpPIDs (Variables|Default|GetPID_Yaw)))
    (:then_2
      (Class|PrimitiveComponent|SetMassOverrideinKg (Variables|Default|GetCollision) "None" (Variables|Static|GetMass) true))
    (:then_3
      (Utilities|IsValid _returnvalue_2
        (:Is%20Valid
          (bind _output_get (Variables|Default|SetAI _returnvalue_2))
          (Utilities|IsValid (Variables|Default|GetTargetObject)
            (:Is%20Valid
              (AI|Components|Blackboard|SetValueasEnum _output_get _returnvalue (Utilities|Enum|LiteralenumCreatureBehavior "NewEnumerator3")))
            (:Is%20Not%20Valid
              (AI|Components|Blackboard|SetValueasEnum _output_get _returnvalue (Utilities|Enum|LiteralenumCreatureBehavior "NewEnumerator1")))))
        (:Is%20Not%20Valid
          (Development|PrintString "NOT VALID BLACKBOARD" true true "(R=0.000000,G=0.660000,B=1.000000,A=1.000000)" 1e+01))))
    (:then_4
      (CallFunction|RepathNewPoint))))

(fn AngleDelta
  (params (θ₁ :type Float%20%28single-precision%29) (θ₂ :type Float%20%28single-precision%29))
  (bind _angle_output (CallFunction|NormalizeAngle θ₁))
  (bind _angle_output_2 (CallFunction|NormalizeAngle θ₂))
  (bind _returnvalue (- _angle_output _angle_output_2))
  (return (Math|Float|SelectFloat (+ _returnvalue 3.6e+02) (Math|Float|SelectFloat (+ _returnvalue -3.6e+02) _returnvalue (> _returnvalue 1.8e+02)) (< _returnvalue -1.8e+02))))

(fn NormalizeAngle
  (params (Angle%20Input :type Float%20%28single-precision%29))
  (return (- Angle%20Input (* (Math|Float|Floor (/ Angle%20Input 3.6e+02)) 3.6e+02))))

(fn GetEulerAngles
  (params (InRot :type Rotator%20%28by%20ref%29))
  (bind (_x _y) (Math|Rotator|BreakRotIntoAxes InRot))
  (bind (_x_2 _y_2) (Math|Vector|BreakVector _x))
  (bind _returnvalue (Class|KismetMathLibrary|DegAtan2 _y_2 _x_2))
  (bind _out (Utilities|*-1 _returnvalue))
  (bind _returnvalue_2 (Math|Vector|RotatorfromAxisandAngle "0, 0,1.000000" _out))
  (bind _returnvalue_3 (Math|Vector|RotateVector _y _returnvalue_2))
  (bind _returnvalue_4 (Math|Vector|RotateVector _x _returnvalue_2))
  (bind (_x_3 _y_3 _z) (Math|Vector|BreakVector _returnvalue_3))
  (bind (_x_4 _y_4 _z_2) (Math|Vector|BreakVector _returnvalue_4))
  (return (Utilities|*-1 (Class|KismetMathLibrary|DegAtan2 _z _y_3)) (Class|KismetMathLibrary|DegAtan2 _z_2 _x_4) _returnvalue (Math|Vector|RotateVector (Math|Vector|MakeVector 0.0 1.0 0.0) (Math|Vector|RotatorfromAxisandAngle "0, 0,1.000000" _returnvalue)) _x))

(fn LerpAngle
  (params (Angle%20A :type Float%20%28single-precision%29) (Angle%20B :type Float%20%28single-precision%29) (Alpha :type Float%20%28single-precision%29))
  (return (+ Angle%20A (* (CallFunction|AngleDelta Angle%20B Angle%20A) Alpha))))

(fn CreatureStatsSetup
  (bind _datatablerowhandle (Utilities|Struct|MakeDataTableRowHandle "/Game/AI/Entities/CreatureTable.CreatureTable" "Default"))
  (bind (_datatable _rowname) (Utilities|Struct|BreakDataTableRowHandle _datatablerowhandle))
  (if (== (.DataTable (Utilities|Struct|BreakDataTableRowHandle (Variables|Static|GetCreatureTableEntry))) "/Game/AI/Entities/CreatureTable.CreatureTable")
    (bind _returnvalue (Utilities|GetDataTableRow (.DataTable (Utilities|Struct|BreakDataTableRowHandle (Variables|Static|GetCreatureTableEntry))) (.RowName (Utilities|Struct|BreakDataTableRowHandle (Variables|Static|GetCreatureTableEntry))))
      (:then
        (LocalVariables|SetCreatureData _returnvalue))
      (:RowNotFound
        (bind _returnvalue_2 (Utilities|GetDataTableRow _datatable _rowname :!label _label)
          (:then
            (LocalVariables|SetCreatureData _returnvalue_2)))))
    (else
      (Variables|Static|SetCreatureTableEntry _datatablerowhandle)
      (goto _label)))
  (Utilities|FlowControl|Sequence
    (:then_0
      (Utilities|FlowControl|Sequence
        (:then_0
          (if (Utilities|Name|Equal(Name) (Variables|Static|GetCreatureName) "None")
            (Variables|Static|SetCreatureName (.ScientificName (Utilities|Struct|BreakCreatureStructure (LocalVariables|GetCreatureData)))))
          (Rendering|Components|TextRender|SetText (Variables|Default|GetLabel) (Utilities|Text|ToText(Name) (Variables|Static|GetCreatureName)))
          (Development|PrintString (Utilities|String|ToString(Text) (Utilities|Text|ToText(Name) (Variables|Static|GetCreatureName))) true true "(R=0.000000,G=0.660000,B=1.000000,A=1.000000)" 1e+01))
        (:then_1
          (Variables|Static|SetMovementInputFrequency (.MovementInputFrequency (Utilities|Struct|BreakCreatureStructure (LocalVariables|GetCreatureData)))))))
    (:then_1
      (return))))