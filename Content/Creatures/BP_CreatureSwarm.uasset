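; Swarm actor that renders many wandering creatures as instances of one mesh.
; Construction scatters instances inside a cloud sphere, sized from a data table row's length range.
; Each tick, every individual eases toward a random point near its origin, pauses on arrival, and smooths yaw and capped pitch.
; Transforms update in one batch, while a smoothed turn amount goes to per-instance custom data.
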(event Custom|Regenerate%20Instances
  (params (New%20Count :type Integer))
  (Components|InstancedStaticMesh|ClearInstances (Variables|Default|GetSwarmInstancer))
  (CallFunction|CreateInstances New%20Count))

(event EventBeginPlay
  (|CallParentFunction) ; This node is disabled and will not be called.\nDrag off pins to build functionality.
)

(event Collision|EventActorBeginOverlap
  (params (OtherActor :type Actor%20Object%20Reference)))

(event EventTick
  (params (DeltaSeconds :type Float%20%28single-precision%29))
  (bind _swarminstancer (Variables|Default|GetSwarmInstancer))
  (|CallParentFunction DeltaSeconds)
  (for (_array_element _array_index) (Variables|Default|GetIndividuals)
    (bind (_return _rotated_amount) (CallFunction|ProcessSingleInstance _array_element DeltaSeconds _array_index))
    (Components|InstancedStaticMesh|SetCustomDataValue _swarminstancer _array_index 0 _rotated_amount false))
  (Class|InstancedStaticMeshComponent|BatchUpdateInstancesTransforms _swarminstancer 0 (Variables|Default|GetTransforms) true false true))

(fn ConstructionScript
  (|CallParentFunction)
  (Utilities|FlowControl|Sequence
    (:then_0
      (if (<= (Variables|Default|GetCloud%20Size) 0.0)
        (Variables|Default|SetCloud%20Size (+ (Math|Conversions|ToFloat(Integer) (Variables|Default|GetSwarm%20Count)) 2e+02))))
    (:then_1
      (Components|Sphere|SetSphereRadius (Variables|Default|GetCloudSize) (Variables|Default|GetCloud%20Size) false))
    (:then_2
      (Components|StaticMesh|SetStaticMesh (Variables|Default|GetSwarmInstancer) (Variables|Default|GetCreature%20Mesh))
      (CallFunction|CreateInstances (Variables|Default|GetSwarm%20Count)))))

(fn RandomVectorinSphere
  (params (Radius :type Float%20%28single-precision%29))
  (bind _output_get (LocalVariables|SetTentative%20Point (Math|Vector|MakeVector (Math|Random|RandomFloatinRange -1.0 1.0) (Math|Random|RandomFloatinRange -1.0 1.0) (Math|Random|RandomFloatinRange -1.0 1.0)) :!label _label))
  (if true
    (return (* (Math|Vector|MakeVector (Utilities|Sign-SafeSquare (.X (Math|Vector|BreakVector _output_get))) (Utilities|Sign-SafeSquare (.Y (Math|Vector|BreakVector _output_get))) (Utilities|Sign-SafeSquare (.Z (Math|Vector|BreakVector _output_get)))) Radius))
    (else
      (goto _label))))

(fn ProcessSingleInstance
  (params (Individual :type Creature%20Swarm%20Individual%20Structure%20%28by%20ref%29) (Delta%20Time :type Float%20%28single-precision%29) (Index :type Integer))
  (bind (_localorigin _currentposition _previousposition _targetposition _rotation _rotationaccumulateddelta _progresstonewpoint) (Utilities|Struct|BreakCreatureSwarmIndividual Individual))
  (bind _pitchcap (Variables|Default|GetPitchCap))
  (bind _transforms (Variables|Default|GetTransforms))
  (bind _returnvalue (Math|Rotator|FindLookatRotation _currentposition _targetposition))
  (bind _output (Utilities|Array|Get(acopy) _transforms Index))
  (bind (_location _rotation_2 _scale) (Math|Transform|BreakTransform _output))
  (Utilities|FlowControl|Sequence
    (:then_0
      (LocalVariables|Setdetla Delta%20Time)
      (LocalVariables|SetNew%20Target _targetposition)
      (if (Math|Vector|Equal(Vector) _targetposition _currentposition 0.001)
        ;[1 1 1] The Individual has arrived at its destination.
        (bind _point (CallFunction|RandomVectorinSphere 5e+01))
        (LocalVariables|SetLocation%20Progress (* (Math|Random|RandomFloat) -3.0))
        (LocalVariables|SetNew%20Target (+ (+ _point _localorigin) (Transformation|GetWorldLocation (Variables|Default|GetCollision))))
        (else
          (LocalVariables|SetLocation%20Progress (+ _progresstonewpoint (* (LocalVariables|Getdetla) 1.0)))))
      (LocalVariables|SetNew%20Individual (Utilities|Struct|MakeCreatureSwarmIndividual _localorigin (Math|Vector|Lerp(Vector) _currentposition _targetposition (Math|Float|Clamp(Float) _progresstonewpoint)) _currentposition (LocalVariables|GetNew%20Target) (Math|Interpolation|RInterpTo _rotation (Math|Rotator|MakeRotator 0.0 0.0 (.Yaw (Math|Rotator|BreakRotator _returnvalue))) (LocalVariables|Getdetla) 6.0) (Math|Float|Lerp (Math|Float|Clamp(Float) (* (Utilities|GetDifferenceBetweenTwoYaws _returnvalue _rotation) 0.01) -1.0) _rotationaccumulateddelta 0.5) (LocalVariables|GetLocation%20Progress))))
    (:then_1
      ;[1 1 1] Update the instance transforms.
      (Utilities|Array|SetArrayElem (Variables|Default|GetTransforms) Index (Math|Transform|MakeTransform (.CurrentPosition (Utilities|Struct|BreakCreatureSwarmIndividual (LocalVariables|GetNew%20Individual))) (Math|Rotator|MakeRotator 0.0 (Math|Float|Clamp(Float) (Math|Float|Lerp (* (- (.Z (Math|Vector|BreakVector (.TargetPosition (Utilities|Struct|BreakCreatureSwarmIndividual (LocalVariables|GetNew%20Individual))))) (.Z (Math|Vector|BreakVector (.CurrentPosition (Utilities|Struct|BreakCreatureSwarmIndividual (LocalVariables|GetNew%20Individual)))))) 0.5) (.Pitch (Math|Rotator|BreakRotator _rotation_2)) 0.9) (* _pitchcap -1.0) _pitchcap) (.Yaw (Math|Rotator|BreakRotator (.Rotation (Utilities|Struct|BreakCreatureSwarmIndividual (LocalVariables|GetNew%20Individual)))))) _scale))
      (Utilities|Array|SetArrayElem (Variables|Default|GetIndividuals) Index (LocalVariables|GetNew%20Individual))
      (return (LocalVariables|GetNew%20Individual) (.RotationAccumulatedDelta (Utilities|Struct|BreakCreatureSwarmIndividual (LocalVariables|GetNew%20Individual)))))))

(fn CreateInstances
  (params (Instance%20Count :type Integer))
  (bind _returnvalue (Math|Random|RandomFloat))
  (bind _creaturetableentry (Variables|Default|GetCreatureTableEntry))
  (bind (_datatable _rowname) (Utilities|Struct|BreakDataTableRowHandle _creaturetableentry))
  (bind _returnvalue_2 (* _returnvalue 3.6e+02))
  (bind _returnvalue_3 (Math|Rotator|MakeRotator 0.0 0.0 _returnvalue_2))
  (for _index (range 0 Instance%20Count)
    (bind _point (CallFunction|RandomVectorinSphere (Variables|Default|GetCloud%20Size)))
    (bind _returnvalue_4 (Utilities|GetDataTableRow _datatable _rowname)
      (:then
        (Components|InstancedStaticMesh|AddInstance (Variables|Default|GetSwarmInstancer) (Math|Transform|MakeTransform _point _returnvalue_3 (Math|Vector|MakeVector (/ (Math|Random|RandomFloatinRange (.X (Math|Vector2D|BreakVector2D (.LengthRange (Utilities|Struct|BreakCreatureStructure _returnvalue_4)))) (.Y (Math|Vector2D|BreakVector2D (.LengthRange (Utilities|Struct|BreakCreatureStructure _returnvalue_4))))) (Variables|Default|GetCreature%20Asset%20Length)) (/ (Math|Random|RandomFloatinRange (.X (Math|Vector2D|BreakVector2D (.LengthRange (Utilities|Struct|BreakCreatureStructure _returnvalue_4)))) (.Y (Math|Vector2D|BreakVector2D (.LengthRange (Utilities|Struct|BreakCreatureStructure _returnvalue_4))))) (Variables|Default|GetCreature%20Asset%20Length)) (/ (Math|Random|RandomFloatinRange (.X (Math|Vector2D|BreakVector2D (.LengthRange (Utilities|Struct|BreakCreatureStructure _returnvalue_4)))) (.Y (Math|Vector2D|BreakVector2D (.LengthRange (Utilities|Struct|BreakCreatureStructure _returnvalue_4))))) (Variables|Default|GetCreature%20Asset%20Length)))))
        (Utilities|Array|Add (Variables|Default|GetTransforms) (Math|Transform|MakeTransform _point _returnvalue_3 (Math|Vector|MakeVector (/ (Math|Random|RandomFloatinRange (.X (Math|Vector2D|BreakVector2D (.LengthRange (Utilities|Struct|BreakCreatureStructure _returnvalue_4)))) (.Y (Math|Vector2D|BreakVector2D (.LengthRange (Utilities|Struct|BreakCreatureStructure _returnvalue_4))))) (Variables|Default|GetCreature%20Asset%20Length)) (/ (Math|Random|RandomFloatinRange (.X (Math|Vector2D|BreakVector2D (.LengthRange (Utilities|Struct|BreakCreatureStructure _returnvalue_4)))) (.Y (Math|Vector2D|BreakVector2D (.LengthRange (Utilities|Struct|BreakCreatureStructure _returnvalue_4))))) (Variables|Default|GetCreature%20Asset%20Length)) (/ (Math|Random|RandomFloatinRange (.X (Math|Vector2D|BreakVector2D (.LengthRange (Utilities|Struct|BreakCreatureStructure _returnvalue_4)))) (.Y (Math|Vector2D|BreakVector2D (.LengthRange (Utilities|Struct|BreakCreatureStructure _returnvalue_4))))) (Variables|Default|GetCreature%20Asset%20Length)))))
        (Utilities|Array|Add (Variables|Default|GetIndividuals) (Utilities|Struct|MakeCreatureSwarmIndividual _point (+ _point (Transformation|GetWorldLocation (Variables|Default|GetCollision))) (+ _point (Transformation|GetWorldLocation (Variables|Default|GetCollision))) (+ _point (Transformation|GetWorldLocation (Variables|Default|GetCollision))) _returnvalue_3 0.0 (Math|Random|RandomFloat))))))
  (return))