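; Player-controlled creature built on a parent creature class, named "PLAYER", with doubled movement speed and acceleration.
; Each tick, movement input rotated by spring-arm yaw becomes a TargetPoint projected from the collision component, while camera input rotates the spring arm.
; BeginPlay attaches a spawned BP_CA_Player; zoom adjusts arm length and Sprint applies a forward impulse.
; Tick also finds UI_VelocityGraph and feeds it combined actor and movement-component speed.
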(event EventBeginPlay
  (|CallParentFunction)
  (bind _returnvalue (Game|SpawnActorfromClass "/Game/CreatureAesthetics/BP_CA_Player.BP_CA_Player_C" (Math|Transform|MakeTransform "0, 0, 0") "Undefined" 0 self))
  (Transformation|AttachActorToActor _returnvalue self "None" "KeepRelative" "KeepRelative" "KeepRelative" true))

(event Collision|EventActorBeginOverlap
  (params (OtherActor :type Actor%20Object%20Reference))
  (|CallParentFunction OtherActor) ; This node is disabled and will not be called.\nDrag off pins to build functionality.
)

(event EventTick
  (params (DeltaSeconds :type Float%20%28single-precision%29))
  (bind _returnvalue (Input|AxisValues|GetMoveForward))
  (bind _returnvalue_2 (Input|AxisValues|GetMoveRight))
  (bind _springarm_0 (Variables|Default|GetSpringArm_0))
  (bind _returnvalue_3 (Math|Vector2D|MakeVector2D _returnvalue _returnvalue_2))
  (bind _relativerotation (Variables|/Script/Engine.SceneComponent|GetRelativeRotation _springarm_0))
  (bind _yaw (Math|Rotator|BreakRotator _relativerotation))
  (bind _returnvalue_4 (Class|KismetMathLibrary|GetRotated2D _returnvalue_3 _yaw))
  (bind (_x _y) (Math|Vector2D|BreakVector2D _returnvalue_4))
  (Variables|Default|SetTargetPoint (+ (* (Math|Vector|MakeVector _x _y (Input|AxisValues|GetMoveUp)) 1e+03) (Transformation|GetWorldLocation (Variables|Default|GetCollision))))
  (|CallParentFunction DeltaSeconds)
  (Utilities|FlowControl|Sequence
    (:then_0
      (Utilities|FlowControl|DoOnce false :!label _label
        (:Completed
          (bind _foundwidgets (Widget|GetAllWidgetsOfClass "/Game/UI/UI_VelocityGraph.UI_VelocityGraph_C" false))
          (Utilities|IsValid (Utilities|Array|Get(acopy) _foundwidgets)
            (:Is%20Valid
              (Variables|Default|SetVelocityGraph (Utilities|Array|Get(acopy) _foundwidgets)))
            (:Is%20Not%20Valid
              (goto _label Reset))))))
    (:then_1
      (Transformation|AddRelativeRotation (Variables|Default|GetSpringArm_0) (Math|Rotator|MakeRotator 0.0 (Input|AxisValues|GetCamUp) (Input|AxisValues|GetCamRight)) false false)
      (Utilities|IsValid (Variables|Default|GetVelocityGraph)
        (:Is%20Valid
          (Default|AddVelocity (Variables|Default|GetVelocityGraph) (+ (Math|Vector|VectorLength (Transformation|GetVelocity self)) (Math|Vector|VectorLength (Variables|/Script/Engine.MovementComponent|GetVelocity (Variables|Default|GetMovementComponent)))) DeltaSeconds))))))

(event Input|ActionEvents|InputActionSprint
  (params (Key :type Key%20Structure :default "None"))
  (:Pressed
    (Physics|AddImpulse (Variables|Default|GetCollision) (* (Math|Vector|Normalize (Transformation|GetActorForwardVector self)) (Math|Float|MakeLiteralFloat 5e+04)) "None" false)))

(event Input|AxisEvents|InputAxisZoomIn
  (params (AxisValue :type Float%20%28single-precision%29))
  (bind _springarm_0 (Variables|Default|GetSpringArm_0))
  (Variables|/Script/Engine.SpringArmComponent|SetTargetArmLength _springarm_0 (Math|Float|Clamp(Float) (+ (* AxisValue -1.0) (Variables|/Script/Engine.SpringArmComponent|GetTargetArmLength _springarm_0)) 2e+02 1e+03)))

(fn ConstructionScript
  (bind _movementcomponent (Variables|Default|GetMovementComponent))
  (|CallParentFunction)
  (bind _output_get (Variables|Default|SetCreatureName "PLAYER"))
  (Rendering|Components|TextRender|SetText (Variables|Default|GetLabel) (Utilities|Text|ToText(Name) _output_get))
  (Variables|/Script/Engine.FloatingPawnMovement|SetMaxSpeed _movementcomponent (* (Variables|/Script/Engine.FloatingPawnMovement|GetMaxSpeed _movementcomponent) 2.0))
  (Variables|/Script/Engine.FloatingPawnMovement|SetAcceleration _movementcomponent (* (Variables|/Script/Engine.FloatingPawnMovement|GetAcceleration _movementcomponent) 2.0)))