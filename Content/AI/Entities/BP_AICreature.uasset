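; AI creature entity Blueprint that is configured through a data table row and a starting behavior.
; On BeginPlay it writes CurrentBehavior to the controller's Blackboard "Behavior" key, then spawns the row's Mesh class as a separate actor attached to itself.
; The construction script sets the label to CreatureName whenever the data table row is found.
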(event EventBeginPlay
  (bind (_bb _key) (Utilities|BlackboardKey "Behavior"))
  (bind _self self)
  (bind _dtrowname (Variables|Static|GetDTRowName))
  (bind (_datatable _rowname) (Utilities|Struct|BreakDataTableRowHandle _dtrowname))
  (|CallParentFunction)
  (AI|Components|Blackboard|SetValueasEnum _bb _key (Variables|Non-Static|GetCurrentBehavior))
  (bind _returnvalue (Utilities|GetDataTableRow _datatable _rowname)
    (:then
      (bind _returnvalue_2 (Game|SpawnActorfromClass (.Mesh (Utilities|Struct|BreakCreatureStructure _returnvalue)) (Math|Transform|MakeTransform "0, 0, 0") "Undefined" _self _self))
      (Transformation|AttachActorToActor _returnvalue_2 self "None" "KeepRelative" "KeepRelative" "KeepRelative" true))))

(event Collision|EventActorBeginOverlap
  (params (OtherActor :type Actor%20Object%20Reference))
  (|CallParentFunction OtherActor) ; This node is disabled and will not be called.\nDrag off pins to build functionality.
)

(event EventTick
  (params (DeltaSeconds :type Float%20%28single-precision%29))
  (|CallParentFunction DeltaSeconds))

(fn ConstructionScript
  (bind _dtrowname (Variables|Static|GetDTRowName))
  (bind (_datatable _rowname) (Utilities|Struct|BreakDataTableRowHandle _dtrowname))
  (|CallParentFunction)
  (bind _returnvalue (Utilities|GetDataTableRow _datatable _rowname)
    (:then
      (Rendering|Components|TextRender|SetText (Variables|Default|GetLabel) (Utilities|Text|ToText(Name) (Variables|Default|GetCreatureName))))))