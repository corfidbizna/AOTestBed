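; Cosmetic ammonite (Metoicoceras) actor attached to a BP_Creature, animating the soft body and static mesh from the creature's movement.
; On Tick it caches the parent creature, with limited retries if none is attached.
; UpdateSquid bends the SquidFlexi spline mesh using yaw-relative heading to SquidTip and vertical velocity, while speed sets the static mesh's roll.
; The construction script initializes the spline short and straight.
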(event Custom|Update%20Squid
  (bind _squidflexi (Variables|Default|GetSquidFlexi))
  (bind _parent_0 (Variables|Default|GetParent_0))
  (bind _squid_length (Variables|Default|GetSquid%20Length))
  (bind _squidtip (Variables|Default|GetSquidTip))
  (bind _squidflexi_2 (Variables|Default|GetSquidFlexi))
  (bind _defaultsceneroot (Variables|Default|GetDefaultSceneRoot))
  (bind _returnvalue (Math|Vector|MakeVector _squid_length 0.0 0.0))
  (bind _returnvalue_2 (Transformation|GetWorldLocation _squidtip))
  (bind _returnvalue_3 (Transformation|GetWorldLocation _squidflexi_2))
  (bind _returnvalue_4 (Transformation|GetWorldRotation _defaultsceneroot))
  (bind _movementcomponent (Variables|/Game/AI/Entities/BP_Creature.BP_Creature_C|GetMovementComponent _parent_0))
  (bind _returnvalue_5 (- _returnvalue_3 _returnvalue_2))
  (bind _yaw (Math|Rotator|BreakRotator _returnvalue_4))
  (bind _velocity (Variables|/Script/Engine.MovementComponent|GetVelocity _movementcomponent))
  (bind _z (Math|Vector|BreakVector _velocity))
  (bind _returnvalue_6 (* _yaw -1.0))
  (bind _returnvalue_7 (Math|Vector|RotateVectorAroundAxis _returnvalue_5 _returnvalue_6 "0, 0,1.000000"))
  (bind _returnvalue_8 (* _z 0.05))
  (bind _returnvalue_9 (Class|KismetMathLibrary|VectorHeadingAngle _returnvalue_7))
  (bind _returnvalue_10 (* _returnvalue_8 4.0))
  (bind _returnvalue_11 (* _returnvalue_9 2e+01))
  (bind _returnvalue_12 (* _returnvalue_11 5.0))
  (bind _returnvalue_13 (Math|Vector|RotateVectorAroundAxis _returnvalue _returnvalue_12 "0, 0,1.000000"))
  (bind _returnvalue_14 (Math|Vector|RotateVectorAroundAxis _returnvalue_13 _returnvalue_10 "0,1.000000, 0"))
  (Utilities|IsValid (Variables|Default|GetParent_0)
    (:Is%20Valid
      (SplineMesh|SetEndPosition _squidflexi (Math|Vector|RotateVectorAroundAxis (Math|Vector|RotateVectorAroundAxis _returnvalue _returnvalue_11 "0, 0,1.000000") _returnvalue_8 "0,1.000000, 0") true)
      (SplineMesh|SetEndTangent _squidflexi _returnvalue_14 true :!class /Script/Engine.SplineMeshComponent)
      (Class|SplineMeshComponent|SetEndRoll _squidflexi (* (.Y (Math|Vector|BreakVector _returnvalue_14)) 0.01) true))))

(event EventTick
  (params (DeltaSeconds :type Float%20%28single-precision%29))
  (bind _self self)
  (bind _returnvalue (Actor|GetAttachParentActor _self))
  (Utilities|FlowControl|Sequence
    (:then_0
      (Utilities|FlowControl|DoOnce false :!label _label
        (:Completed
          (Utilities|IsValid _returnvalue
            (:Is%20Valid
              (bind _asbp_creature (Utilities|Casting|CastToBP_Creature _returnvalue)
                (:then
                  (Variables|Default|SetParent_0 _asbp_creature))
                (:CastFailed
                  (Development|PrintString "Got parent, but it wasn't a Creature."))))
            (:Is%20Not%20Valid
              (Development|PrintString "Parent doesn't exist. ")
              (Utilities|FlowControl|DoN 10
                (:Exit
                  (goto _label Reset))))))))
    (:then_1
      (Utilities|IsValid (Variables|Default|GetParent_0)
        (:Is%20Valid
          (CallFunction|UpdateSquid)
          (Transformation|SetRelativeRotation (Variables|Default|GetStaticMesh) (Math|Rotator|MakeRotator (Math|Float|MapRangeClamped (Math|Vector|VectorLength (Variables|/Script/Engine.MovementComponent|GetVelocity (Variables|/Game/AI/Entities/BP_Creature.BP_Creature_C|GetMovementComponent (Variables|Default|GetParent_0)))) 0.0 3e+02 1.3e+02 1e+02) 0.0 -9e+01) false false))))))

(fn ConstructionScript
  (bind _squidflexi (Variables|Default|GetSquidFlexi))
  (bind _squid_length (Variables|Default|GetSquid%20Length))
  (bind _returnvalue (* _squid_length 0.1))
  (bind _returnvalue_2 (Math|Vector|MakeVector _returnvalue 0.0 0.0))
  (|CallParentFunction)
  (SplineMesh|SetEndPosition _squidflexi _returnvalue_2 true)
  (SplineMesh|SetEndTangent _squidflexi _returnvalue_2 true :!class /Script/Engine.SplineMeshComponent))