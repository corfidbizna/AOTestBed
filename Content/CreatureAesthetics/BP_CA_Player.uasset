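; Player creature aesthetics actor that animates a squid's shell and siphon from the movement of its attached parent BP_Creature.
; On Tick it looks up and caches that parent once, retrying a limited number of times if none exists.
; Speed then pitches the shell, opens the SiphonClosed morph target as it rises, and continually accumulates into PercentMaxSpeed.
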(event EventTick
  (params (DeltaSeconds :type Float%20%28single-precision%29))
  (bind _self self)
  (bind _returnvalue (Actor|GetAttachParentActor _self))
  (|CallParentFunction DeltaSeconds)
  (Utilities|FlowControl|Sequence
    (:then_0
      (Utilities|FlowControl|DoOnce false :!label _label
        (:Completed
          (Utilities|IsValid _returnvalue
            (:Is%20Valid
              (bind _asbp_creature (Utilities|Casting|CastToBP_Creature _returnvalue)
                (:then
                  (Variables|Default|SetParent_0 _asbp_creature))
                (:CastFailed
                  (Development|PrintString "Got parent, but it wasn't a Creature."))))
            (:Is%20Not%20Valid
              (Development|PrintString "Parent doesn't exist. ")
              (Utilities|FlowControl|DoN 10
                (:Exit
                  (goto _label Reset))))))))
    (:then_1
      (Utilities|IsValid (Variables|Default|GetParent_0)
        (:Is%20Valid
          (Transformation|SetRelativeRotation (Variables|Default|GetShell) (Math|Rotator|MakeRotator -9e+01 (Math|Float|MapRangeClamped (Math|Vector|VectorLength (Variables|/Script/Engine.MovementComponent|GetVelocity (Variables|/Game/AI/Entities/BP_Creature.BP_Creature_C|GetMovementComponent (Variables|Default|GetParent_0)))) 0.0 3e+02 -6e+01 -85.0) 1.8e+02) false false)
          (Variables|Default|SetPercentMaxSpeed (+ (Variables|Default|GetPercentMaxSpeed) (* (Math|Vector|VectorLength (+ (Variables|/Script/Engine.MovementComponent|GetVelocity (Variables|/Game/AI/Entities/BP_Creature.BP_Creature_C|GetMovementComponent (Variables|Default|GetParent_0))) (Transformation|GetVelocity (Variables|Default|GetParent_0)))) 0.001))))))
    (:then_2
      (Components|SkeletalMesh|SetMorphTarget (Variables|Default|GetSquidSkeleton) "SiphonClosed" (Math|Float|MapRangeClamped (Math|Vector|VectorLength (+ (Variables|/Script/Engine.MovementComponent|GetVelocity (Variables|/Game/AI/Entities/BP_Creature.BP_Creature_C|GetMovementComponent (Variables|Default|GetParent_0))) (Transformation|GetVelocity (Variables|Default|GetParent_0)))) 0.0 5e+02 1.0 0.0) true))))

(fn ConstructionScript
  (|CallParentFunction))