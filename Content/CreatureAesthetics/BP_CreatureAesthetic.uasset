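; BP_CreatureAesthetic tracks the movement state of the BP_Creature it belongs to, apparently as a base for creature visuals.
; On Tick it resolves Parent by casting its instigator, retrying until valid.
; It then derives speed as a fraction of max speed, vertical velocity, and the per-frame yaw change of the creature's collision component.
; The yaw change is a raw difference, without angle wrapping or delta-time scaling.
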(event EventBeginPlay)

(event EventTick
  (params (DeltaSeconds :type Float%20%28single-precision%29))
  (Utilities|FlowControl|Sequence
    (:then_0
      ;[1 1 1] Parent Setup
      (Utilities|IsValid (Variables|Default|GetParent)
        (:Is%20Not%20Valid
          (bind _asbp_creature (Utilities|Casting|CastToBP_Creature (Game|GetInstigator)))
          (Variables|Default|SetParent _asbp_creature))))
    (:then_1
      (Variables|Default|SetPercentMaxSpeed (/ (Math|Vector|VectorLength (Variables|/Script/Engine.MovementComponent|GetVelocity (Pawn|GetMovementComponent (Variables|Default|GetParent)))) (Class|MovementComponent|GetMaxSpeed (Pawn|GetMovementComponent (Variables|Default|GetParent)))))
      (Variables|Default|SetVelocityVertical (.Z (Math|Vector|BreakVector (Variables|/Script/Engine.MovementComponent|GetVelocity (Pawn|GetMovementComponent (Variables|Default|GetParent))))))
      (Variables|Default|SetVelocityYaw (- (.Yaw (Default|GetEulerAngles (Variables|Default|GetParent) (Transformation|GetWorldRotation (Variables|/Game/AI/Entities/BP_Creature.BP_Creature_C|GetCollision (Variables|Default|GetParent))))) (Variables|Default|GetYawLastFrame)))
      (Variables|Default|SetYawLastFrame (.Yaw (Default|GetEulerAngles (Variables|Default|GetParent) (Transformation|GetWorldRotation (Variables|/Game/AI/Entities/BP_Creature.BP_Creature_C|GetCollision (Variables|Default|GetParent)))))))))

(fn ConstructionScript)