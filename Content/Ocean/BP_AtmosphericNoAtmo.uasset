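; Ocean atmosphere Blueprint that switches underwater look by geological era and keeps marine snow ahead of the camera.
; SwitchEra, also run at construction, reads fog and depth values from a data table and swaps the ambient light cubemap for non-Default eras.
; It also sets caustics parameters in a material collection and snow count.
; Fog values are only stored, as the nodes applying them are unconnected; Tick repositions the snow using camera yaw.
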(event Custom|Switch%20Era
  (params (NewParam :type Enum_Periods%20Enum :default "NewEnumerator0"))
  (Variables|Default|SetPeriod%20Preset NewParam)
  (Utilities|FlowControl|Sequence
    (:then_0
      ;[1 1 1] Atmosphere Setup
      (bind _returnvalue (Utilities|GetDataTableRow "/Game/Ocean/PeriodAtmoData.PeriodAtmoData" (Utilities|String|StringToName (Utilities|String|EnumtoString (Variables|Default|GetPeriod%20Preset))))
        (:then
          (if (Utilities|Enum|NotEqual(Enum) (Variables|Default|GetPeriod%20Preset) "NewEnumerator0")
            (Utilities|FlowControl|Sequence
              (:then_0
                (Variables|Atmosphere|SetFog%20Color (.FogTint (Utilities|Struct|BreakStruct_PeriodSettings _returnvalue)))
                (Variables|Atmosphere|SetFog%20Thickness (.FogThickness (Utilities|Struct|BreakStruct_PeriodSettings _returnvalue))))
              (:then_1
                (Variables|Atmosphere|SetDepth%20Tint (.DepthTint (Utilities|Struct|BreakStruct_PeriodSettings _returnvalue)))
                (Variables|Atmosphere|SetDepth%20Start%20Distance (.DepthStartDistance (Utilities|Struct|BreakStruct_PeriodSettings _returnvalue))))
              (:then_2
                (Class|SkyLightComponent|SetCubemap (Variables|Default|GetLightAmbient) (Utilities|Select :Index (Variables|Default|GetPeriod%20Preset) :NewEnumerator0 "/Game/Ocean/reflections/reflection_00.reflection_00" :NewEnumerator1 "/Game/Ocean/reflections/reflection_00.reflection_00" :NewEnumerator2 "/Game/Ocean/reflections/reflection_01.reflection_01" :NewEnumerator3 "/Game/Ocean/reflections/reflection_02.reflection_02" :NewEnumerator4 "/Game/Ocean/reflections/reflection_03.reflection_03" :NewEnumerator5 "/Game/Ocean/reflections/reflection_04.reflection_04" :NewEnumerator6 "/Game/Ocean/reflections/reflection_05.reflection_05" :NewEnumerator7 "/Game/Ocean/reflections/reflection_06.reflection_06" :NewEnumerator8 "/Game/Ocean/reflections/reflection_07.reflection_07"))))))))
    (:then_1
      (Rendering|Material|SetScalarParameterValue "/Game/Materials/MC_OceanThings.MC_OceanThings" "Caustics Speed" (Variables|Lighting|GetRefraction%20Speed) :!class /Script/Engine.KismetMaterialLibrary)
      (Rendering|Material|SetScalarParameterValue "/Game/Materials/MC_OceanThings.MC_OceanThings" "Caustics Amount" (Variables|Lighting|GetRefraction%20Strength) :!class /Script/Engine.KismetMaterialLibrary)
      (Effects|Components|ParticleSystem|SetFloatParameter (Variables|Default|GetMarineSnow) "Count" (* (Variables|Atmosphere|GetSnow%20Density) 0.01)))
    (:then_2
      (Development|ExecuteConsoleCommand "r.ReflectionCapture" 0))))

(event EventTick
  (params (DeltaSeconds :type Float%20%28single-precision%29))
  (bind _returnvalue (Game|GetPlayerCameraManager 0))
  (Transformation|SetWorldLocation (Variables|Default|GetMarineSnow) (+ (Math|Vector|RotateVectorAroundAxis (Math|Vector|MakeVector 5e+02 0.0 0.0) (.Yaw (Math|Rotator|BreakRotator (Camera|GetCameraRotation _returnvalue))) "0.000000, 0,1.000000") (Camera|GetCameraLocation _returnvalue)) false false))

(fn ConstructionScript
  (CallFunction|SwitchEra (Variables|Default|GetPeriod%20Preset)))