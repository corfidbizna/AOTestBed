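; BP_DoodadPopulator is a construction-script actor that scatters doodad meshes over surfaces inside an adjustable box volume.
; The Doods map supplies meshes and counts to up to three instanced mesh components.
; Random downward Visibility traces place fixed-scale instances with X axes along hit normals, retrying misses without limit.
; A one-shot SnapToWorldGrid toggle calls a grid-rounding function whose rounding math is left unconnected.
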(event EventBeginPlay)

(event Collision|EventActorBeginOverlap
  (params (OtherActor :type Actor%20Object%20Reference)))

(event EventTick
  (params (DeltaSeconds :type Float%20%28single-precision%29)))

(fn ConstructionScript
  (bind _self self)
  (bind _box (Variables|Default|GetBox))
  (bind _height (Variables|Default|GetHeight))
  (bind _dood00 (Variables|Default|GetDood00))
  (bind _dood01 (Variables|Default|GetDood01))
  (bind _dood02 (Variables|Default|GetDood02))
  (bind _width (Variables|Default|GetWidth))
  (bind _doods (Variables|Default|GetDoods))
  (bind _returnvalue (* _width 0.5))
  (bind _returnvalue_2 (* _height 0.5))
  (bind _array (Utilities|Array|MakeArray _dood00 _dood01 _dood02))
  (bind _defaultsceneroot (Variables|Default|GetDefaultSceneRoot _self))
  (bind _returnvalue_3 (Transformation|GetWorldLocation _defaultsceneroot))
  (bind (_x _y _z) (Math|Vector|BreakVector _returnvalue_3))
  (Utilities|FlowControl|Sequence
    (:then_0
      (if (Variables|Default|GetSnapToWorldGrid)
        (Transformation|SetWorldLocation _defaultsceneroot (Math|Vector|MakeVector (Utilities|RoundtoWorldGridatWidth _x) (Utilities|RoundtoWorldGridatWidth _y) _z) false false)
        (Variables|Default|SetSnapToWorldGrid false)))
    (:then_1
      (Components|Box|SetBoxExtent _box (Math|Vector|MakeVector _returnvalue _returnvalue _returnvalue_2) false)
      (Transformation|SetRelativeLocation _box (Math|Vector|MakeVector 0.0 0.0 _returnvalue_2) false false))
    (:then_2
      (bind _keys (Utilities|Map|Keys _doods))
      (bind (_array_element _array_index) (Utilities|Array|ForEachLoopwithBreak _keys :!label _label)
        (:LoopBody
          (if (< _array_index (Utilities|Array|Length _array))
            (bind _values (Utilities|Map|Values _doods))
            (Components|StaticMesh|SetStaticMesh (Utilities|Array|Get(acopy) _array _array_index) _array_element)
            (bind _instancetransforms (CallFunction|GenerateTransformsforInstances (Utilities|Array|Get(acopy) _values _array_index)))
            (Components|InstancedStaticMesh|AddInstances (Utilities|Array|Get(acopy) _array _array_index) _instancetransforms false)
            (else
              (goto _label Break))))))))

(fn GenerateTransformsforInstances
  (params (Count :type Integer))
  (bind _width (Variables|Default|GetWidth))
  (bind _returnvalue (* _width 0.5))
  (bind _returnvalue_2 (* _width -0.5))
  (while (< (LocalVariables|GetIndex) Count)
    (bind _output_get (LocalVariables|SetTraceStart (Math|Vector|MakeVector (Math|Random|RandomFloatinRange _returnvalue_2 _returnvalue) (Math|Random|RandomFloatinRange _returnvalue_2 _returnvalue) (Variables|Default|GetHeight))))
    (bind (_outhit _returnvalue_3) (Collision|LineTraceByChannel (+ _output_get (Transformation|GetWorldLocation (Variables|Default|GetDefaultSceneRoot self))) (- (+ _output_get (Transformation|GetWorldLocation (Variables|Default|GetDefaultSceneRoot self))) (Math|Vector|MakeVector 0.0 0.0 (Variables|Default|GetHeight))) "TraceTypeQuery1" false 0 "None"))
    (if _returnvalue_3
      (Utilities|Array|Add (LocalVariables|GetTransforms) (Math|Transform|MakeTransform (- (LocalVariables|GetTraceStart) (Math|Vector|MakeVector 0.0 0.0 (.Distance (Collision|BreakHitResult _outhit)))) (Math|Conversions|RotationFromXVector (.Normal (Collision|BreakHitResult _outhit))) "5.000000,5.000000,5.000000"))
      (Math|Integer|IncrementInt (LocalVariables|GetIndex))))
  (return (LocalVariables|GetTransforms)))