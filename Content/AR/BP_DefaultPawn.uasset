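; BP_DefaultPawn is a pawn in the AR folder whose BeginPlay, Tick, Possessed and Unpossessed events are all empty.
; Disconnected logic would find or spawn a BP_AquariumEnviron and cache it as Environ.
; Other unwired chains would show that environment only while this pawn is player 0's pawn, and toggle its non-AR visibility.
; None of this logic runs, and the construction script is empty.
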(event EventBeginPlay)

(event EventTick
  (params (DeltaSeconds :type Float%20%28single-precision%29)))

(event EventPossessed
  (params (NewController :type Controller%20Object%20Reference)))

(event EventUnpossessed
  (params (OldController :type Controller%20Object%20Reference)))

(fn ConstructionScript)