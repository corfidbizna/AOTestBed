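; AR pawn for an ocean creature experience that runs the AR session and provides the space creatures swim in.
; Possession and unpossession request AR status changes from OceanState, while separate events start and stop floor-tracked AR sessions.
; Tick finds the AR interface widget and feeds it session status.
; Creatures leaving CoordinateBounds repath immediately, and point requests are delegated to the BP_AquariumRegions child actor.
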(event OnComponentEndOverlap(CoordinateBounds)
  (params (OverlappedComponent :type Primitive%20Component%20Object%20Reference) (OtherActor :type Actor%20Object%20Reference) (OtherComp :type Primitive%20Component%20Object%20Reference) (OtherBodyIndex :type Integer))
  (bind _asbp_creature (Utilities|Casting|CastToBP_Creature OtherActor))
  (Default|RepathNewPoint _asbp_creature))

(event EventBeginPlay
  (bind _asocean_state (Utilities|Casting|CastToOceanState (Game|GetGameState) :!label _label)
    (:then
      (Variables|Default|SetGameState _asocean_state))
    (:CastFailed
      (Utilities|FlowControl|DoN 10
        (:Exit
          (goto _label))))))

(event EventTick
  (params (DeltaSeconds :type Float%20%28single-precision%29))
  (Utilities|FlowControl|Sequence
    (:then_0
      (Utilities|IsValid (Variables|Default|GetInterfaceWidget)
        (:Is%20Valid
          (Default|UpdateARStatus (Variables|Default|GetInterfaceWidget) (Class|ARBlueprintLibrary|GetARSessionStatus)))
        (:Is%20Not%20Valid
          (bind _foundwidgets (Widget|GetAllWidgetsOfClass "/Game/AR/UI_ARInterface.UI_ARInterface_C" true))
          (Variables|Default|SetInterfaceWidget (Utilities|Array|Get(acopy) _foundwidgets)))))))

(event EventUnpossessed
  (params (OldController :type Controller%20Object%20Reference))
  (bind _gamestate (Variables|Default|GetGameState))
  (Utilities|IsValid _gamestate
    (:Is%20Valid
      (Default|AttemptARStatusChange _gamestate false))))

(event EventPossessed
  (params (NewController :type Controller%20Object%20Reference))
  (bind _gamestate (Variables|Default|GetGameState))
  (Utilities|IsValid _gamestate
    (:Is%20Valid
      (Default|AttemptARStatusChange _gamestate true))))

(event Custom|AR%20End
  (Class|ARBlueprintLibrary|StopARSession))

(event Custom|AR%20Attempt%20Start
  (bind _returnvalue (Class|ARBlueprintLibrary|GetARSessionStatus))
  (bind _interfacewidget (Variables|Default|GetInterfaceWidget))
  (Class|HeadMountedDisplayFunctionLibrary|SetTrackingOrigin "Floor")
  (Class|ARBlueprintLibrary|StartARSession "/Game/AR/ARSessionConfig.ARSessionConfig")
  (Utilities|FlowControl|Sequence
    (:then_0
      (Utilities|IsValid _interfacewidget
        (:Is%20Valid
          (Default|UpdateARStatus _interfacewidget _returnvalue))))
    (:then_1
      (switch Utilities|FlowControl|Switch|SwitchonEARSessionStatus (.Status (Utilities|Struct|BreakARSessionStatus _returnvalue))))))

(fn ConstructionScript)

(fn GetPointInsideCoordinateBounds
  (bind _asbp_aquarium_regions (Utilities|Casting|CastToBP_AquariumRegions (Variables|/Script/Engine.ChildActorComponent|GetChildActor (Variables|Default|GetCoordinates))))
  (return (Default|GetPointInsideCoordinateBounds _asbp_aquarium_regions)))