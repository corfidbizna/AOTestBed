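; BP_AquariumRegions is an AR actor that defines a box region and supplies random points within its bounds, apparently for aquarium content.
; The construction script sizes the Region00 box from the Dimensions variable.
; GetPointInsideCoordinateBounds picks a random point using the box's relative location and extent, then rotates that vector around Z by the box's world yaw, without adding actor location.
; The event graph holds only disabled stub events.
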(event EventBeginPlay)

(event Collision|EventActorBeginOverlap
  (params (OtherActor :type Actor%20Object%20Reference)))

(event EventTick
  (params (DeltaSeconds :type Float%20%28single-precision%29)))

(fn ConstructionScript
  (Components|Box|SetBoxExtent (Variables|Default|GetRegion00) (Variables|Default|GetDimensions) false))

(fn GetPointInsideCoordinateBounds
  (bind _region00 (Variables|Default|GetRegion00))
  (return (Math|Vector|RotateVectorAroundAxis (Math|Random|RandomPointinBoundingBox (Variables|/Script/Engine.SceneComponent|GetRelativeLocation _region00) (Variables|/Script/Engine.BoxComponent|GetBoxExtent _region00)) (.Yaw (Math|Rotator|BreakRotator (Transformation|GetWorldRotation _region00))) "0, 0,1.000000")))